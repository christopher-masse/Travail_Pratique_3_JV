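; BP_Door is an interactable hinged door that toggles open and closed on Interact.
; A DoorState value (Open, Opening, Closed, Closing) gates Open and Close, allowing a toggle mid-swing.
; One timeline rotates the Pivot's yaw between zero and Angle, and its direction on finish sets the final state.
; Closing reverses from the current position, while opening always plays from start, even when interrupting a close.
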(event `/Game/Blueprints/BPI_Interactible.Interact`
  (`self.Toggle`))

(event `OpenDoor`
  (set `self.DoorState` "NewEnumerator2")
  (bind (_direction _alpha) (`Timeline|TL_Door_Opening` :!via `PlayFromStart` :!label _label)
    (:`Update`
      (`SceneComponent.K2_SetRelativeRotation` (`self.Pivot`) (`KismetMathLibrary.MakeRotator` 0.0 0.0 (`KismetMathLibrary.Lerp` 0.0 (`self.Angle`) _alpha)) false false))
    (:`Finished`
      (switch `ETimelineDirection` _direction
        (:`Forward`
          (set `self.DoorState` "NewEnumerator0"))
        (:`Backward`
          (set `self.DoorState` "NewEnumerator1"))))))

(event `CloseDoor`
  (set `self.DoorState` "NewEnumerator3")
  (goto _label :!via `Reverse`))

(fn `Close`
  (switch `/Game/Blueprints/E_DoorState` (`self.DoorState`)
    (:`NewEnumerator0`
      _)
    (:`NewEnumerator2`
      _))
  (`self.CloseDoor`))

(fn `Open`
  (switch `/Game/Blueprints/E_DoorState` (`self.DoorState`)
    (:`NewEnumerator1`
      _)
    (:`NewEnumerator3`
      _))
  (`self.OpenDoor`))

(fn `Toggle`
  (switch `/Game/Blueprints/E_DoorState` (`self.DoorState`)
    (:`NewEnumerator0`
      (`self.Close` :!label _label))
    (:`NewEnumerator1`
      (`self.Open` :!label _label_2))
    (:`NewEnumerator2`
      (goto _label))
    (:`NewEnumerator3`
      (goto _label_2))))

(fn `UserConstructionScript`)